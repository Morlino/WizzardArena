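; Slime King boss enemy that periodically unleashes a slam area-of-effect attack against wizard characters.
; Tick accumulates a timer and plays the King AOE montage each time the cooldown elapses.
; A separate PerformAOE event, not called within this graph, shakes the camera and damages wizards found by a sphere overlap whose radius scales with the actor's X scale.
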(event Custom|PerformAOE
  (Camera|PlayWorldCameraShake "/Game/Game/Blueprints/Characters/Enemy/Slime/Boss/BP_KingSlamShake.BP_KingSlamShake_C" (Transformation|GetActorLocation) 0.0 1e+04)
  (bind _output_get (Variables|Default|SetAOE_ActualRadius (* (.x (Transformation|GetActorScale3D)) (Variables|Default|GetAOE_Radius))))
  (bind _outactors (Collision|SphereOverlapActors (Transformation|GetActorLocation) (Variables|Default|GetAOE_ActualRadius) (Utilities|Array|MakeArray "ObjectTypeQuery3") 0 (Utilities|Array|MakeArray self)))
  (for _array_element _outactors
    (bind _asbp_wizzard_character (Utilities|Casting|CastToBP_WizzardCharacter _array_element))
    (Game|Damage|ApplyDamage _asbp_wizzard_character (Variables|Default|GetAOE_Damage) 0 0)))

(event EventBeginPlay
  (|CallParentFunction) ; This node is disabled and will not be called.\nDrag off pins to build functionality.
)

(event Collision|EventActorBeginOverlap
  (params (OtherActor :type Actor%20Object%20Reference))
  (|CallParentFunction OtherActor) ; This node is disabled and will not be called.\nDrag off pins to build functionality.
)

(event EventTick
  (params (DeltaSeconds :type Float%20%28single-precision%29))
  (bind _output_get (Variables|Default|SetAOE_Timer (+ DeltaSeconds (Variables|Default|GetAOE_Timer))))
  (if (>= _output_get (Variables|Default|GetAOE_Cooldown))
    (Animation|PlayAnimMontage "/Game/Game/Blueprints/Characters/Enemy/Slime/Animations/AM_KingAOE.AM_KingAOE" 1.0 "None")
    (Variables|Default|SetAOE_Timer 0.0)))

(fn ConstructionScript
  (|CallParentFunction))