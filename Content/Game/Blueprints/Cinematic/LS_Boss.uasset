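; Sequencer event Blueprint for the LS_Boss cinematic, handing control between gameplay and the boss sequence.
; Begin hides the wizard player, turns off its collision, disables input, removes the gameplay mapping context and hides the HUD.
; End restores character, mapping context and HUD, without calling EnableInput.
; It then starts the WaveManager's next wave and moves the Slime King and player to the locations of sequence-bound actors.
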(event Custom|End
  (bind _asbp_wizzard_character (Utilities|Casting|CastToBP_WizzardCharacter (Game|GetPlayerCharacter 0)))
  (Collision|SetActorEnableCollision _asbp_wizzard_character true)
  (Rendering|SetActorHiddenInGame _asbp_wizzard_character false)
  (Input|AddMappingContext (PlayerController|LocalPlayerSubsystems|GetEnhancedInputLocalPlayerSubsystem (Game|GetPlayerController 0)) "/Game/Game/Inputs/IMC_Gameplay.IMC_Gameplay" 0 "(bIgnoreAllPressedKeysUntilRelease=True,bForceImmediately=False,bNotifyUserSettings=False)")
  (bind _foundwidgets (Widget|GetAllWidgetsOfClass "/Game/Game/Blueprints/Widgets/WBP_WizzardHUD.WBP_WizzardHUD_C" true))
  (for _array_element _foundwidgets
    _)
  (Widget|SetVisibility _array_element "Visible")
  (bind _returnvalue (Actor|GetActorOfClass "/Script/WizzardArena.WaveManager"))
  (Class|WaveManager|StartNextWave _returnvalue)
  (bind _returnvalue_2 (Class|LevelSequenceDirector|GetBoundActor (|GetSequenceBinding)))
  (bind _returnvalue_3 (Actor|GetActorOfClass "/Game/Game/Blueprints/Characters/Enemy/Slime/Boss/BP_SlimeKing.BP_SlimeKing_C"))
  (Transformation|SetActorLocation _returnvalue_3 (Transformation|GetActorLocation _returnvalue_2) false false)
  (bind _returnvalue_4 (Class|LevelSequenceDirector|GetBoundActor (|GetSequenceBinding)))
  (Transformation|SetActorLocation (Game|GetPlayerCharacter 0) (Transformation|GetActorLocation _returnvalue_4) false false))

(event Custom|Begin
  (bind _returnvalue (Game|GetPlayerController 0))
  (bind _asbp_wizzard_character (Utilities|Casting|CastToBP_WizzardCharacter (Game|GetPlayerCharacter 0)))
  (Collision|SetActorEnableCollision _asbp_wizzard_character false)
  (Rendering|SetActorHiddenInGame _asbp_wizzard_character true)
  (Input|DisableInput _returnvalue _returnvalue)
  (Input|RemoveMappingContext (PlayerController|LocalPlayerSubsystems|GetEnhancedInputLocalPlayerSubsystem (Game|GetPlayerController 0)) "/Game/Game/Inputs/IMC_Gameplay.IMC_Gameplay" "(bIgnoreAllPressedKeysUntilRelease=True,bForceImmediately=False,bNotifyUserSettings=False)")
  (bind _foundwidgets (Widget|GetAllWidgetsOfClass "/Game/Game/Blueprints/Widgets/WBP_WizzardHUD.WBP_WizzardHUD_C" true))
  (for _array_element _foundwidgets
    (Widget|SetVisibility _array_element "Hidden")))